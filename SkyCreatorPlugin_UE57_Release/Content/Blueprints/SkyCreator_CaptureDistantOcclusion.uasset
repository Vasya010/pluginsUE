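; Sky Creator actor meant to capture a top-down distant occlusion heightmap into a render target and share its placement with materials.
; The construction script assigns the render target, sizes the ortho capture and box from CaptureWidth, and stores corner and center positions.
; It and BeginPlay call the parameter and capture functions, but both are empty.
; Their scene capture and MPC_SC_Common writes sit unconnected, so neither runs.
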(event EventBeginPlay
  (CallFunction|SetParameterCollectionValues)
  (SkyCreator|CaptureHeightmap))

(fn ConstructionScript
  (bind _capturewidth (Variables|SkyCreator|GetCaptureWidth))
  (bind _returnvalue (/ _capturewidth 2.0))
  (bind _returnvalue_2 (Math|Vector|MakeVector _returnvalue _returnvalue 0.0))
  (Variables|/Script/Engine.SceneCaptureComponent2D|SetTextureTarget (Variables|Default|GetOcclusionDistantCapture) (Variables|SkyCreator|GetRenderTarget))
  (Variables|/Script/Engine.SceneCaptureComponent2D|SetOrthoWidth (Variables|Default|GetOcclusionDistantCapture) (Variables|SkyCreator|GetCaptureWidth))
  (Components|Box|SetBoxExtent (Variables|Default|GetBox) _returnvalue_2 true)
  (Variables|SkyCreator|SetCapturePosition (- (Transformation|GetActorLocation) _returnvalue_2))
  (Variables|SkyCreator|SetCaptureCenterPosition (Transformation|GetActorLocation))
  (CallFunction|SetParameterCollectionValues)
  (SkyCreator|CaptureHeightmap))

(fn CaptureHeightmap)

(fn SetParameterCollectionValues)