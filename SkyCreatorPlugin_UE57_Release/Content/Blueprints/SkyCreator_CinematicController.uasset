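; Cinematic controller actor that drives the SkyCreator sky's time of day and weather.
; Its construction script finds the SkyCreator actor in the level and applies the current settings.
; Each tick it sets the sky's Time and blends between two weather presets by an interpolation alpha.
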(event EventTick
  (params (DeltaSeconds :type Float%20%28single-precision%29))
  (CallFunction|UpdateTimeandWeather))

(fn ConstructionScript
  (bind _returnvalue (Actor|GetActorOfClass "/Script/SkyCreatorPlugin.SkyCreator"))
  (Variables|Default|SetSkyCreatorTarget _returnvalue)
  (CallFunction|UpdateTimeandWeather))

(fn UpdateTimeandWeather
  (Utilities|IsValid (Variables|Default|GetSkyCreatorTarget)
    (:Is%20Valid
      (Class|SkyCreator|SetTime (Variables|Default|GetSkyCreatorTarget) (Variables|Time|GetTime))
      (Class|SkyCreator|LerpWeatherSettings (Variables|Default|GetSkyCreatorTarget) (Class|SkyCreatorWeatherPreset|GetWeatherPresetSettings (Variables|Weather|GetWeatherPresetA)) (Class|SkyCreatorWeatherPreset|GetWeatherPresetSettings (Variables|Weather|GetWeatherPresetB)) (Variables|Weather|GetInterpolationAlpha)))))