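; SkyCreator_SimpleWeatherChange is a helper actor that previews weather and time changes on the level's SkyCreator sky.
; Its construction script finds the SkyCreator actor and, when weather override is on, lerps between two weather presets by an alpha.
; An optional time override, applied only alongside the weather override, also sets the sky's time.
; BeginPlay does nothing, so all logic runs at construction.
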(event EventBeginPlay)

(fn ConstructionScript
  (bind _returnvalue (Actor|GetActorOfClass "/Script/SkyCreatorPlugin.SkyCreator"))
  (Variables|Default|SetSkyCreatorTarget _returnvalue)
  (Utilities|IsValid (Variables|Default|GetSkyCreatorTarget)
    (:Is%20Valid
      (if (Variables|Default|GetOverrideWeather)
        (Class|SkyCreator|LerpWeatherSettings (Variables|Default|GetSkyCreatorTarget) (Class|SkyCreatorWeatherPreset|GetWeatherPresetSettings (Variables|Default|GetWeatherPresetA)) (Class|SkyCreatorWeatherPreset|GetWeatherPresetSettings (Variables|Default|GetWeatherPresetB)) (Variables|Default|GetAlpha))
        (if (Variables|Default|GetOverrideTime)
          (Class|SkyCreator|SetTime (Variables|Default|GetSkyCreatorTarget) (Variables|Default|GetTime)))))))