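; Example controller for the level's SkyCreator actor, running real-time time of day and random weather changes on the authority.
; Random-interval timers start blends to random weather presets with optional random wind, lerped in Tick from timer elapsed time.
; Changed wetness, puddle and snow amounts can start separate accumulate or dry/melt timers that drive material FX lerps.
; It also feeds rain and wind audio parameters and plays distance-based lightning or thunder sounds.
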(event Custom|Start_WeatherChangeInterval
  ;[0 0 0] Weather Change Interval
  (Networking|SwitchHasAuthority
    (:Authority
      (Utilities|Time|ClearandInvalidateTimerbyHandle (Variables|Weather|GetTimer_WeatherChangeInterval))
      (Variables|Weather|SetCurrentChangeInterval (Math|Random|RandomFloatinRange (Variables|Weather|GetChangeIntervalTimeMin) (Variables|Weather|GetChangeIntervalTimeMax)))
      (bind _returnvalue (Utilities|Time|SetTimerbyEvent (EventDispatchers|CreateEvent :!event Custom|Finish_WeatherChangeInterval) (Variables|Weather|GetCurrentChangeInterval)))
      (Variables|Weather|SetTimer_WeatherChangeInterval _returnvalue))))

(event Custom|Start_WeatherInterpolation
  ;[0 0 0] Weather Interpolation example using Timers.
  ; Chooses random weather preset from an array to interpolate to.
  ; You can call "Start_WeatherInterpolation" on any time.
  (Networking|SwitchHasAuthority
    (:Authority
      (if (not (Utilities|Time|IsTimerActivebyHandle (Variables|Weather|GetTimer_WeatherInterpolateDuration)))
        (Utilities|Time|ClearandInvalidateTimerbyHandle (Variables|Weather|GetTimer_WeatherInterpolateDuration))
        (Variables|Weather|SetWeatherInterpolateDuration (Math|Random|RandomFloatinRange (Variables|Weather|GetInterpolateDurationTimeMin) (Variables|Weather|GetInterpolateDurationTimeMax)))
        (bind _returnvalue (Utilities|Time|SetTimerbyEvent (EventDispatchers|CreateEvent :!event Custom|Finish_WeatherInterpolation) (Variables|Weather|GetWeatherInterpolateDuration))) ; Activates interpolation timer
        (Variables|Weather|SetTimer_WeatherInterpolateDuration _returnvalue)
        (Variables|Weather|SetCurrentWeatherSettings (Class|SkyCreator|GetWeatherSettings (Variables|Default|GetSkyCreatorTarget)))
        (Variables|Wind|SetCurrentWindSettings (Class|SkyCreator|GetWindSettings (Variables|Default|GetSkyCreatorTarget)))
        (Variables|Weather|SetNextWeatherPreset (Utilities|Array|Get(acopy) (Variables|Weather|GetRandomWeatherPresets) (Math|Random|RandomIntegerinRange 0 (- (Utilities|Array|Length (Variables|Weather|GetRandomWeatherPresets)) 1))))
        (Variables|Weather|SetNextWeatherSettings (Class|SkyCreatorWeatherPreset|GetWeatherPresetSettings (Variables|Weather|GetNextWeatherPreset)))
        (Variables|Wind|SetCurrentWindDirection (Math|Random|RandomFloatinRange 0.0 3.6e+02))
        (Variables|Wind|SetCurrentCloudWindDirection (Math|Random|RandomFloatinRange 0.0 3.6e+02))
        (bind _structout (Utilities|Struct|SetmembersinSkyCreatorWindSettings (.WindSettings (Utilities|Struct|BreakSkyCreatorWeatherSettings (Variables|Weather|GetNextWeatherSettings))) (Variables|Wind|GetCurrentCloudWindDirection) (Variables|Wind|GetCurrentWindDirection)))
        (Variables|Wind|SetNextWindSettings _structout)
        (Development|PrintString (Utilities|String|Append "Started Weather Interpolation to a Weather Preset: " (Utilities|GetDisplayName (Variables|Weather|GetNextWeatherPreset))) (Variables|Default|GetDrawDebugMessages) false "(R=0.000000,G=0.658824,B=1.000000,A=1.000000)" 4.0)
        (Utilities|FlowControl|Sequence
          (:then_0
            (Variables|WeatherMaterialFX|SetCurrentWetnessAmount (Utilities|GetWetnessAmount (Variables|Weather|GetCurrentWeatherSettings)))
            (Variables|WeatherMaterialFX|SetNextWetnessAmount (Utilities|GetWetnessAmount (Variables|Weather|GetNextWeatherSettings)))
            (if (!= (Variables|WeatherMaterialFX|GetCurrentWetnessAmount) (Variables|WeatherMaterialFX|GetNextWetnessAmount))
              (Utilities|FlowControl|Sequence
                (:then_0
                  (if (< (Variables|WeatherMaterialFX|GetCurrentWetnessAmount) (Variables|WeatherMaterialFX|GetNextWetnessAmount))
                    (CallFunction|StartWetnessAccumulate)))
                (:then_1
                  (if (== (Variables|WeatherMaterialFX|GetNextWetnessAmount) 0.0)
                    (CallFunction|StartWetnessDry))))))
          (:then_1
            (Variables|WeatherMaterialFX|SetCurrentPuddlesAmount (Utilities|GetPuddlesAmount (Variables|Weather|GetCurrentWeatherSettings)))
            (Variables|WeatherMaterialFX|SetNextPuddlesAmount (Utilities|GetPuddlesAmount (Variables|Weather|GetNextWeatherSettings)))
            (if (!= (Variables|WeatherMaterialFX|GetCurrentPuddlesAmount) (Variables|WeatherMaterialFX|GetNextPuddlesAmount))
              (Utilities|FlowControl|Sequence
                (:then_0
                  (if (< (Variables|WeatherMaterialFX|GetCurrentPuddlesAmount) (Variables|WeatherMaterialFX|GetNextPuddlesAmount))
                    (CallFunction|StartPuddlesAccumulate)))
                (:then_1
                  (if (== (Variables|WeatherMaterialFX|GetNextPuddlesAmount) 0.0)
                    (CallFunction|StartPuddlesDry))))))
          (:then_2
            (Variables|WeatherMaterialFX|SetCurrentSnowAmount (Utilities|GetSnowAmount (Variables|Weather|GetCurrentWeatherSettings)))
            (Variables|WeatherMaterialFX|SetNextSnowAmount (Utilities|GetSnowAmount (Variables|Weather|GetNextWeatherSettings)))
            (if (!= (Variables|WeatherMaterialFX|GetCurrentSnowAmount) (Variables|WeatherMaterialFX|GetNextSnowAmount))
              (Utilities|FlowControl|Sequence
                (:then_0
                  (if (< (Variables|WeatherMaterialFX|GetCurrentSnowAmount) (Variables|WeatherMaterialFX|GetNextSnowAmount))
                    (CallFunction|StartSnowAccumulate)))
                (:then_1
                  (if (== (Variables|WeatherMaterialFX|GetNextSnowAmount) 0.0)
                    (CallFunction|StartSnowMelt)))))))
        (else
          (Development|PrintString "Weather Interpolation is in progress" (Variables|Default|GetDrawDebugMessages) false "(R=1.000000,G=0.366667,B=0.000000,A=1.000000)" 4.0))))))

(event Custom|Finish_WetnessAccumulation
  ;[0 0 0] Material FX interpolation using Timers.
  ; In this setup this calls automatically when Wetness, Puddles or Snow amounts are different between Current and Next Weather Preset.
  (Utilities|Time|ClearandInvalidateTimerbyHandle (Variables|WeatherMaterialFX|GetWetnessAccumulationTimer)))

(event Custom|Finish_SnowDry
  ;[0 0 0] Material FX interpolation using Timers.
  ; In this setup this calls automatically when Wetness, Puddles or Snow amounts are different between Current and Next Weather Preset.
  (Utilities|Time|ClearandInvalidateTimerbyHandle (Variables|WeatherMaterialFX|GetSnowMeltTimer)))

(event Custom|Start_WetnessAccumulate
  ;[0 0 0] Material FX interpolation using Timers.
  ; In this setup this calls automatically when Wetness, Puddles or Snow amounts are different between Current and Next Weather Preset.
  (Networking|SwitchHasAuthority
    (:Authority
      (Utilities|Time|ClearandInvalidateTimerbyHandle (Variables|WeatherMaterialFX|GetWetnessAccumulationTimer))
      (bind _returnvalue (Utilities|Time|SetTimerbyEvent (EventDispatchers|CreateEvent :!event Custom|Finish_WetnessAccumulation) (Variables|WeatherMaterialFX|GetWetnessAccumulateDuration)))
      (Variables|WeatherMaterialFX|SetWetnessAccumulationTimer _returnvalue))))

(event Custom|Start_WetnessDry
  ;[0 0 0] Material FX interpolation using Timers.
  ; In this setup this calls automatically when Wetness, Puddles or Snow amounts are different between Current and Next Weather Preset.
  (Networking|SwitchHasAuthority
    (:Authority
      (Utilities|Time|ClearandInvalidateTimerbyHandle (Variables|WeatherMaterialFX|GetWetnessDryTimer))
      (bind _returnvalue (Utilities|Time|SetTimerbyEvent (EventDispatchers|CreateEvent :!event Custom|Finish_WetnessDry) (Variables|WeatherMaterialFX|GetWetnessDryDuration)))
      (Variables|WeatherMaterialFX|SetWetnessDryTimer _returnvalue))))

(event Custom|Start_PuddlesAccumulate
  ;[0 0 0] Material FX interpolation using Timers.
  ; In this setup this calls automatically when Wetness, Puddles or Snow amounts are different between Current and Next Weather Preset.
  (Networking|SwitchHasAuthority
    (:Authority
      (Utilities|Time|ClearandInvalidateTimerbyHandle (Variables|WeatherMaterialFX|GetPuddlesAccumulationTimer))
      (bind _returnvalue (Utilities|Time|SetTimerbyEvent (EventDispatchers|CreateEvent :!event Custom|Finish_PuddlesAccumulation) (Variables|WeatherMaterialFX|GetPuddlesAccumulateDuration)))
      (Variables|WeatherMaterialFX|SetPuddlesAccumulationTimer _returnvalue))))

(event Custom|Start_SnowMelt
  ;[0 0 0] Material FX interpolation using Timers.
  ; In this setup this calls automatically when Wetness, Puddles or Snow amounts are different between Current and Next Weather Preset.
  (Networking|SwitchHasAuthority
    (:Authority
      (Utilities|Time|ClearandInvalidateTimerbyHandle (Variables|WeatherMaterialFX|GetSnowMeltTimer))
      (bind _returnvalue (Utilities|Time|SetTimerbyEvent (EventDispatchers|CreateEvent :!event Custom|Finish_PuddlesDry) (Variables|WeatherMaterialFX|GetPuddlesDryDuration)))
      (Variables|WeatherMaterialFX|SetSnowMeltTimer _returnvalue))))

(event Custom|Start_PuddlesDry
  ;[0 0 0] Material FX interpolation using Timers.
  ; In this setup this calls automatically when Wetness, Puddles or Snow amounts are different between Current and Next Weather Preset.
  (Networking|SwitchHasAuthority
    (:Authority
      (Utilities|Time|ClearandInvalidateTimerbyHandle (Variables|WeatherMaterialFX|GetPuddlesDryTimer))
      (bind _returnvalue (Utilities|Time|SetTimerbyEvent (EventDispatchers|CreateEvent :!event Custom|Finish_PuddlesDry) (Variables|WeatherMaterialFX|GetPuddlesDryDuration)))
      (Variables|WeatherMaterialFX|SetPuddlesDryTimer _returnvalue))))

(event Custom|Finish_WeatherInterpolation
  ;[0 0 0] Weather Interpolation example using Timers.
  ; Chooses random weather preset from an array to interpolate to.
  ; You can call "Start_WeatherInterpolation" on any time.
  (Utilities|Time|ClearandInvalidateTimerbyHandle (Variables|Weather|GetTimer_WeatherInterpolateDuration))
  (Variables|Weather|SetCurrentWeatherSettings (Variables|Weather|GetNextWeatherSettings))
  (Development|PrintString "Weather Interpolation is finished" (Variables|Default|GetDrawDebugMessages) false "(R=0.016667,G=1.000000,B=0.000000,A=1.000000)" 4.0)
  (if (Variables|Weather|GetbRealtimeWeatherChange)
    (CallFunction|StartWeatherChangeInterval)))

(event Custom|Start_SnowAccumulate
  ;[0 0 0] Material FX interpolation using Timers.
  ; In this setup this calls automatically when Wetness, Puddles or Snow amounts are different between Current and Next Weather Preset.
  (Networking|SwitchHasAuthority
    (:Authority
      (Utilities|Time|ClearandInvalidateTimerbyHandle (Variables|WeatherMaterialFX|GetSnowAccumulationTimer))
      (bind _returnvalue (Utilities|Time|SetTimerbyEvent (EventDispatchers|CreateEvent :!event Custom|Finish_PuddlesDry) (Variables|WeatherMaterialFX|GetPuddlesDryDuration)))
      (Variables|WeatherMaterialFX|SetSnowAccumulationTimer _returnvalue))))

(event Custom|Finish_PuddlesDry
  ;[0 0 0] Material FX interpolation using Timers.
  ; In this setup this calls automatically when Wetness, Puddles or Snow amounts are different between Current and Next Weather Preset.
  (Utilities|Time|ClearandInvalidateTimerbyHandle (Variables|WeatherMaterialFX|GetPuddlesDryTimer)))

(event Custom|Finish_SnowAccumulate
  ;[0 0 0] Material FX interpolation using Timers.
  ; In this setup this calls automatically when Wetness, Puddles or Snow amounts are different between Current and Next Weather Preset.
  (Utilities|Time|ClearandInvalidateTimerbyHandle (Variables|WeatherMaterialFX|GetSnowAccumulationTimer)))

(event Custom|Finish_WeatherChangeInterval
  ;[0 0 0] Weather Change Interval
  (Utilities|Time|ClearandInvalidateTimerbyHandle (Variables|Weather|GetTimer_WeatherChangeInterval))
  (CallFunction|StartWeatherInterpolation))

(event Custom|LightningStrike
  (params (LightningPosition :type Vector))
  ;[0 0 0] Example how to spawn Lightning Sound
  (if (<= (Math|Vector|Distance(Vector) LightningPosition (Camera|GetCameraLocation (Game|GetPlayerCameraManager 0))) 2e+06)
    (Audio|SpawnSound2D "/SkyCreatorPlugin/Sounds/Lightning/A_SC_Lightning_Cue.A_SC_Lightning_Cue" 0.5 1.0 0.0 0)
    (else
      (Audio|SpawnSound2D "/SkyCreatorPlugin/Sounds/Lightning/A_SC_Thunder_Cue.A_SC_Thunder_Cue" 0.5 1.0 0.0 0))))

(event Custom|Finish_WetnessDry
  ;[0 0 0] Material FX interpolation using Timers.
  ; In this setup this calls automatically when Wetness, Puddles or Snow amounts are different between Current and Next Weather Preset.
  (Utilities|Time|ClearandInvalidateTimerbyHandle (Variables|WeatherMaterialFX|GetWetnessDryTimer)))

(event Custom|Finish_PuddlesAccumulation
  ;[0 0 0] Material FX interpolation using Timers.
  ; In this setup this calls automatically when Wetness, Puddles or Snow amounts are different between Current and Next Weather Preset.
  (Utilities|Time|ClearandInvalidateTimerbyHandle (Variables|WeatherMaterialFX|GetPuddlesAccumulationTimer)))

(event EventBeginPlay
  ;[0 0 0] Begin Play
  (Networking|SwitchHasAuthority
    (:Authority
      (Utilities|FlowControl|Sequence
        (:then_0
          (EventDispatchers|BindEventtoOnLightningStrike (Variables|Default|GetSkyCreatorTarget) (EventDispatchers|CreateEvent :!event Custom|LightningStrike))
          (if (Variables|Time|GetbRealtimeTimeOfDay)
            (Class|SkyCreator|SetTime (Variables|Default|GetSkyCreatorTarget) (Variables|Time|GetRealtimeTimeOfDayStart))))
        (:then_1
          (if (Variables|Weather|GetbRealtimeWeatherChange)
            (Class|SkyCreator|SetWeatherSettings (Variables|Default|GetSkyCreatorTarget) (Class|SkyCreatorWeatherPreset|GetWeatherPresetSettings (Variables|Weather|GetStartWeatherPreset)))
            (if (Variables|Weather|GetbRealtimeWeatherChange)
              (CallFunction|StartWeatherChangeInterval))))))
    (:Remote
      (CallFunction|SetAudioRainAmount)
      (CallFunction|SetAudioWindAmount))))

(event EventTick
  (params (DeltaSeconds :type Float%20%28single-precision%29))
  ;[0 0 0] Tick
  (Networking|SwitchHasAuthority
    (:Authority
      (Development|PrintString (Utilities|String|ToString(Float) (Class|SkyCreator|GetTime (Variables|Default|GetSkyCreatorTarget))) (Variables|Default|GetDrawDebugMessages) false "(R=0.000000,G=0.658824,B=1.000000,A=1.000000)" (Utilities|Time|GetWorldDeltaSeconds))
      (Utilities|FlowControl|Sequence
        (:then_0
          (if (Variables|Time|GetbRealtimeTimeOfDay)
            (Class|SkyCreator|RealtimeTimeOfDay (Variables|Default|GetSkyCreatorTarget) (Utilities|Time|GetWorldDeltaSeconds) (Variables|Time|GetRealtimeTimeOfDayDuration))))
        (:then_1
          (if (Utilities|Time|IsTimerActivebyHandle (Variables|Weather|GetTimer_WeatherInterpolateDuration)) ; "Lerp Weather Settings" function \nwill tick when Timer is Active
            (Variables|Weather|SetInterpolateDurationAlpha (Math|Float|MapRangeClamped (Class|KismetSystemLibrary|GetTimerElapsedTimeHandle (Variables|Weather|GetTimer_WeatherInterpolateDuration)) 0.0 (Variables|Weather|GetWeatherInterpolateDuration) 0.0 1.0))
            (Development|PrintString (Utilities|String|Append "Interpolating Weather...  " (Utilities|String|ToString(Float) (Utilities|Time|GetTimerRemainingTimebyHandle (Variables|Weather|GetTimer_WeatherInterpolateDuration)))) (Variables|Default|GetDrawDebugMessages) false "(R=0.000000,G=0.658824,B=1.000000,A=1.000000)" (Utilities|Time|GetWorldDeltaSeconds))
            (Class|SkyCreator|LerpWeatherSettings (Variables|Default|GetSkyCreatorTarget) (Variables|Weather|GetCurrentWeatherSettings) (Variables|Weather|GetNextWeatherSettings) (Variables|Weather|GetInterpolateDurationAlpha))
            (if (Variables|Wind|GetbEnableRandomWind)
              (Class|SkyCreator|LerpWindSettings (Variables|Default|GetSkyCreatorTarget) (Variables|Wind|GetCurrentWindSettings) (Variables|Wind|GetNextWindSettings) (Variables|Weather|GetInterpolateDurationAlpha)))))
        (:then_2
          (CallFunction|MaterialFXInterpolation)
          (if (not (Networking|IsDedicatedServer))
            (CallFunction|SetAudioRainAmount)
            (CallFunction|SetAudioWindAmount)))))
    (:Remote
      (CallFunction|SetAudioRainAmount)
      (CallFunction|SetAudioWindAmount))))

(fn ConstructionScript
  (bind _returnvalue (Actor|GetActorOfClass "/Script/SkyCreatorPlugin.SkyCreator"))
  (Variables|Default|SetSkyCreatorTarget _returnvalue))

(fn MaterialFXInterpolation
  (Utilities|FlowControl|Sequence
    (:then_0
      (if (Utilities|Time|IsTimerActivebyHandle (Variables|WeatherMaterialFX|GetWetnessAccumulationTimer))
        (Class|SkyCreator|LerpWetnessAmount (Variables|Default|GetSkyCreatorTarget) (Variables|WeatherMaterialFX|GetCurrentWetnessAmount) (Variables|WeatherMaterialFX|GetNextWetnessAmount) (Math|Float|MapRangeClamped (Class|KismetSystemLibrary|GetTimerElapsedTimeHandle (Variables|WeatherMaterialFX|GetWetnessAccumulationTimer)) 0.0 (Variables|WeatherMaterialFX|GetWetnessAccumulateDuration) 0.0 1.0))
        (Development|PrintString (Utilities|String|Append "Accumulate Wetness Timer: " (Utilities|String|ToString(Float) (Utilities|Time|GetTimerRemainingTimebyHandle (Variables|WeatherMaterialFX|GetWetnessAccumulationTimer)))) (Variables|Default|GetDrawDebugMessages) false "(R=0.000000,G=0.658824,B=1.000000,A=1.000000)" (Utilities|Time|GetWorldDeltaSeconds))))
    (:then_1
      (if (Utilities|Time|IsTimerActivebyHandle (Variables|WeatherMaterialFX|GetWetnessDryTimer))
        (Class|SkyCreator|LerpWetnessAmount (Variables|Default|GetSkyCreatorTarget) (Variables|WeatherMaterialFX|GetCurrentWetnessAmount) (Variables|WeatherMaterialFX|GetNextWetnessAmount) (Math|Float|MapRangeClamped (Class|KismetSystemLibrary|GetTimerElapsedTimeHandle (Variables|WeatherMaterialFX|GetWetnessDryTimer)) 0.0 (Variables|WeatherMaterialFX|GetWetnessDryDuration) 0.0 1.0))
        (Development|PrintString (Utilities|String|Append "Dry Wetness Timer: " (Utilities|String|ToString(Float) (Utilities|Time|GetTimerRemainingTimebyHandle (Variables|WeatherMaterialFX|GetWetnessDryTimer)))) (Variables|Default|GetDrawDebugMessages) false "(R=0.000000,G=0.658824,B=1.000000,A=1.000000)" (Utilities|Time|GetWorldDeltaSeconds))))
    (:then_2
      (if (Utilities|Time|IsTimerActivebyHandle (Variables|WeatherMaterialFX|GetPuddlesAccumulationTimer))
        (Class|SkyCreator|LerpPuddlesAmount (Variables|Default|GetSkyCreatorTarget) (Variables|WeatherMaterialFX|GetCurrentPuddlesAmount) (Variables|WeatherMaterialFX|GetNextPuddlesAmount) (Math|Float|MapRangeClamped (Class|KismetSystemLibrary|GetTimerElapsedTimeHandle (Variables|WeatherMaterialFX|GetPuddlesAccumulationTimer)) 0.0 (Variables|WeatherMaterialFX|GetPuddlesAccumulateDuration) 0.0 1.0))
        (Development|PrintString (Utilities|String|Append "Accumule Puddles Timer: " (Utilities|String|ToString(Float) (Utilities|Time|GetTimerRemainingTimebyHandle (Variables|WeatherMaterialFX|GetPuddlesAccumulationTimer)))) (Variables|Default|GetDrawDebugMessages) false "(R=0.000000,G=0.658824,B=1.000000,A=1.000000)" (Utilities|Time|GetWorldDeltaSeconds))))
    (:then_3
      (if (Utilities|Time|IsTimerActivebyHandle (Variables|WeatherMaterialFX|GetPuddlesDryTimer))
        (Class|SkyCreator|LerpPuddlesAmount (Variables|Default|GetSkyCreatorTarget) (Variables|WeatherMaterialFX|GetCurrentPuddlesAmount) (Variables|WeatherMaterialFX|GetNextPuddlesAmount) (Math|Float|MapRangeClamped (Class|KismetSystemLibrary|GetTimerElapsedTimeHandle (Variables|WeatherMaterialFX|GetPuddlesDryTimer)) 0.0 (Variables|WeatherMaterialFX|GetPuddlesDryDuration) 0.0 1.0))
        (Development|PrintString (Utilities|String|Append "Dry Puddles Timer: " (Utilities|String|ToString(Float) (Utilities|Time|GetTimerRemainingTimebyHandle (Variables|WeatherMaterialFX|GetPuddlesDryTimer)))) (Variables|Default|GetDrawDebugMessages) false "(R=0.000000,G=0.658824,B=1.000000,A=1.000000)" (Utilities|Time|GetWorldDeltaSeconds))))
    (:then_4
      (if (Utilities|Time|IsTimerActivebyHandle (Variables|WeatherMaterialFX|GetSnowAccumulationTimer))
        (Class|SkyCreator|LerpSnowAmount (Variables|Default|GetSkyCreatorTarget) (Variables|WeatherMaterialFX|GetCurrentSnowAmount) (Variables|WeatherMaterialFX|GetNextSnowAmount) (Math|Float|MapRangeClamped (Class|KismetSystemLibrary|GetTimerElapsedTimeHandle (Variables|WeatherMaterialFX|GetSnowAccumulationTimer)) 0.0 (Variables|WeatherMaterialFX|GetSnowAccumulateDuration) 0.0 1.0))
        (Development|PrintString (Utilities|String|Append "Accumulate Snow Timer: " (Utilities|String|ToString(Float) (Utilities|Time|GetTimerRemainingTimebyHandle (Variables|WeatherMaterialFX|GetSnowAccumulationTimer)))) (Variables|Default|GetDrawDebugMessages) false "(R=0.000000,G=0.658824,B=1.000000,A=1.000000)" (Utilities|Time|GetWorldDeltaSeconds))))
    (:then_5
      (if (Utilities|Time|IsTimerActivebyHandle (Variables|WeatherMaterialFX|GetSnowMeltTimer))
        (Class|SkyCreator|LerpSnowAmount (Variables|Default|GetSkyCreatorTarget) (Variables|WeatherMaterialFX|GetCurrentSnowAmount) (Variables|WeatherMaterialFX|GetNextSnowAmount) (Math|Float|MapRangeClamped (Class|KismetSystemLibrary|GetTimerElapsedTimeHandle (Variables|WeatherMaterialFX|GetSnowMeltTimer)) 0.0 (Variables|WeatherMaterialFX|GetSnowMeltDuration) 0.0 1.0))
        (Development|PrintString (Utilities|String|Append "Melt Snow Timer: " (Utilities|String|ToString(Float) (Utilities|Time|GetTimerRemainingTimebyHandle (Variables|WeatherMaterialFX|GetSnowMeltTimer)))) (Variables|Default|GetDrawDebugMessages) false "(R=0.000000,G=0.658824,B=1.000000,A=1.000000)" (Utilities|Time|GetWorldDeltaSeconds))))))

(fn SetAudioRainAmount
  (Audio|Parameter|SetFloatParameter (Variables|Default|GetSoundRain) "RainAmount" (.RainAmount (Utilities|Struct|BreakSkyCreatorWeatherFXSettings (Class|SkyCreator|GetWeatherFXSettings (Variables|Default|GetSkyCreatorTarget)))) :!class /Script/AudioExtensions.AudioParameterControllerInterface))

(fn SetAudioWindAmount
  (Audio|Parameter|SetFloatParameter (Variables|Default|GetSoundWind) "WindAmount" (.WindSpeed (Utilities|Struct|BreakSkyCreatorWindSettings (Class|SkyCreator|GetWindSettings (Variables|Default|GetSkyCreatorTarget)))) :!class /Script/AudioExtensions.AudioParameterControllerInterface))